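; BP_MC is a character Blueprint handling move, attack, parry and dash, with movement and dashing along the Y axis.
; Move stores the input as DesiredLocation and feeds its Y into movement, while Attack and Parry only print debug messages.
; Dash, gated by InputLocked and a DoOnce, line-traces along the stored direction.
; A Timeline then interpolates actor location over DashDistance, clamping Y just short of any blocking hit.
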(event Custom|Move
  (params (ActionValue :type Vector%202D%20Structure))
  ;[1 1 1] Move Event
  (bind _output_get (Variables|Movement|SetDesired%20Location ActionValue))
  (CallFunction|PrintDebugMessage "X" "X= " (Utilities|String|ToString(Float) (.x _output_get)) "" 2.0)
  (CallFunction|PrintDebugMessage "Y" "Y= " (Utilities|String|ToString(Float) (.y _output_get)) "" 2.0)
  (Pawn|Input|AddMovementInput (Math|Vector|MakeVector 0.0 (.y _output_get) 0.0) 1.0 false))

(event Custom|Attack
  ;[1 1 1] Attack Event
  (CallFunction|PrintDebugMessage "Attack" "" "Attacking " (Utilities|String|ToString(Vector2d) (Variables|Movement|GetDesired%20Location)) 1.0))

(event Custom|Parry
  ;[1 1 1] Parry Event
  (CallFunction|PrintDebugMessage "Attack" "" "Parrying " (Utilities|String|ToString(Vector2d) (Variables|Movement|GetDesired%20Location)) 1.0))

(event Custom|Dash
  ;[1 1 1] Dash, Gate and Setting up Variables
  (if (not (Variables|Movement|GetInputLocked?))
    (Utilities|FlowControl|DoOnce false :!label _label
      (:Completed
        (Variables|Movement|SetDashStartVector (Transformation|GetActorLocation))
        ;;[1 1 1] LineTrace
        (Variables|Movement|SetDash%20Direction%20Vector (Math|Vector|Normalize (Math|Vector|MakeVector 0.0 (.y (Variables|Movement|GetDesired%20Location)) 0.0)))
        (bind _outhit (Collision|LineTraceByChannel (Variables|Movement|GetDashStartVector) (+ (* (Variables|Movement|GetDash%20Direction%20Vector) (Variables|Movement|GetDash%20Distance)) (Variables|Movement|GetDashStartVector)) "TraceTypeQuery1" false 0 "Persistent"))
        (Variables|Movement|SetDashTraceHitResult _outhit)
        ;[1 1 1] Vector Logic
        (bind _distancepercantage (Timeline|Timeline PlayFromStart)
          (:Update
            (if (not (.bBlockingHit (Collision|BreakHitResult (Variables|Movement|GetDashTraceHitResult))))
              (Transformation|SetActorLocation (Math|Vector|MakeVector (.x (+ (* (* (Variables|Movement|GetDash%20Direction%20Vector) (Variables|Movement|GetDash%20Distance)) _distancepercantage) (Variables|Movement|GetDashStartVector))) (.y (+ (* (* (Variables|Movement|GetDash%20Direction%20Vector) (Variables|Movement|GetDash%20Distance)) _distancepercantage) (Variables|Movement|GetDashStartVector))) (.z (+ (* (* (Variables|Movement|GetDash%20Direction%20Vector) (Variables|Movement|GetDash%20Distance)) _distancepercantage) (Variables|Movement|GetDashStartVector)))) false false)
              (else
                ;[1 1 1] Clamp maximum distance based on hit result of line trace
                (if (< (.y (.ImpactPoint (Collision|BreakHitResult (Variables|Movement|GetDashTraceHitResult)))) (.y (Variables|Movement|GetDashStartVector)))
                  (Transformation|SetActorLocation (Math|Vector|MakeVector (.x (+ (* (* (Variables|Movement|GetDash%20Direction%20Vector) (Variables|Movement|GetDash%20Distance)) _distancepercantage) (Variables|Movement|GetDashStartVector))) (- (Math|Float|Clamp(Float) (.y (+ (* (* (Variables|Movement|GetDash%20Direction%20Vector) (Variables|Movement|GetDash%20Distance)) _distancepercantage) (Variables|Movement|GetDashStartVector))) (.y (.ImpactPoint (Collision|BreakHitResult (Variables|Movement|GetDashTraceHitResult)))) 0.0) -1e+01) (.z (+ (* (* (Variables|Movement|GetDash%20Direction%20Vector) (Variables|Movement|GetDash%20Distance)) _distancepercantage) (Variables|Movement|GetDashStartVector)))) false false)
                  (else
                    (Transformation|SetActorLocation (Math|Vector|MakeVector (.x (+ (* (* (Variables|Movement|GetDash%20Direction%20Vector) (Variables|Movement|GetDash%20Distance)) _distancepercantage) (Variables|Movement|GetDashStartVector))) (+ (Math|Float|Clamp(Float) (.y (+ (* (* (Variables|Movement|GetDash%20Direction%20Vector) (Variables|Movement|GetDash%20Distance)) _distancepercantage) (Variables|Movement|GetDashStartVector))) 0.0 (.y (.ImpactPoint (Collision|BreakHitResult (Variables|Movement|GetDashTraceHitResult))))) -1e+01) (.z (+ (* (* (Variables|Movement|GetDash%20Direction%20Vector) (Variables|Movement|GetDash%20Distance)) _distancepercantage) (Variables|Movement|GetDashStartVector)))) false false))))))
          (:Finished
            (Variables|Movement|SetInputLocked? false)
            (goto _label Reset)))))))

(fn ConstructionScript)