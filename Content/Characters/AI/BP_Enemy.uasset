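; BP_Enemy is an enemy character that reports its health to the player's controller for a health bar.
; On BeginPlay it caches player controller 0 as BP_MCPC, sets current health to max, then UpdateHealthbar writes the health ratio to that controller's EnemyHealthPercent.
; An AI move toward the player character is present but unwired, so it never runs.
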(event EventBeginPlay
  (bind _asbp_mcpc (Utilities|Casting|CastToBP_MCPC (Game|GetPlayerController 0)))
  (Variables|References|SetPlayerController_Ref _asbp_mcpc)
  (Variables|Default|SetCurrentHealth (Variables|Default|GetMaxHealth))
  (CallFunction|UpdateHealthbar))

(fn ConstructionScript)

(fn UpdateHealthbar
  (Variables|/Game/Game/BP_MCPC.BP_MCPC_C|SetEnemyHealthPercent (Variables|References|GetPlayerController_Ref) (/ (Variables|Default|GetCurrentHealth) (Variables|Default|GetMaxHealth)))
  (return))