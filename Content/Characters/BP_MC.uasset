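; Player character for a side-scrolling action game moving along the Y axis, with dash, directional attack and parry, wall run and wall jump.
; An enum state tracks the current action, with montages gating attack and parry.
; Timelines drive wall runs and line-trace-clamped dashes, while attacks and parries only cast debug-drawn sphere traces.
; A looping timer lowers stance after a post-damage delay; a debug key applies test damage.
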(event OnComponentBeginOverlap(WallDetection)
  (params (OverlappedComponent :type Primitive%20Component%20Object%20Reference) (OtherActor :type Actor%20Object%20Reference) (OtherComp :type Primitive%20Component%20Object%20Reference) (OtherBodyIndex :type Integer) (bFromSweep :type Boolean) (SweepResult :type Hit%20Result%20Structure%20%28by%20ref%29))
  ;[1 1 1] WallRun
  (bind _asstatic_mesh_component (Utilities|Casting|CastToStaticMeshComponent OtherComp))
  (Utilities|IsValid (Variables|Movement|GetClimbed%20Object)
    (:Is%20Valid
      (if (== (Variables|Movement|GetClimbed%20Object) _asstatic_mesh_component)
        _
        (else
          (Variables|Movement|SetCanRunOnWalls? true)
          (Variables|Movement|SetClimbed%20Object _asstatic_mesh_component :!label _label))))
    (:Is%20Not%20Valid
      (goto _label)))
  (if (Utilities|Enum|Equal(Enum) (Variables|Default|GetStateMachine) "NewEnumerator2")
    (if (Variables|Movement|GetCanRunOnWalls?)
      (Utilities|FlowControl|DoOnce false
        (:Completed
          (Variables|Movement|SetCanRunOnWalls? false)
          (Variables|Default|SetStateMachine "NewEnumerator5")
          (Timeline|Wall%20Run%20Duration PlayFromStart
            (:Update
              (Variables|/Script/Engine.MovementComponent|SetVelocity (Variables|Character|GetCharacterMovement) (Math|Vector|MakeVector (.x (Variables|/Script/Engine.MovementComponent|GetVelocity (Variables|Character|GetCharacterMovement))) (.y (Variables|/Script/Engine.MovementComponent|GetVelocity (Variables|Character|GetCharacterMovement))) (Variables|Movement|GetWallRunSpeed))))
            (:Finished
              (CallFunction|WallRunCancel))))))))

(event OnComponentEndOverlap(WallDetection)
  (params (OverlappedComponent :type Primitive%20Component%20Object%20Reference) (OtherActor :type Actor%20Object%20Reference) (OtherComp :type Primitive%20Component%20Object%20Reference) (OtherBodyIndex :type Integer))
  ;[1 1 1] WallRun
  (if (== OtherComp (Variables|Movement|GetClimbed%20Object))
    (CallFunction|WallRunCancel)))

(event Custom|Move
  (params (ActionValue :type Vector%202D%20Structure))
  ;[1 1 1] Move Event
  (bind _output_get (Variables|Default|SetDesired%20Location ActionValue))
  (CallFunction|PrintDebugMessage "X" "X= " (Utilities|String|ToString(Float) (.x _output_get)) "" 2.0 "(R=0.000000,G=1.000000,B=1.000000,A=1.000000)")
  (CallFunction|PrintDebugMessage "Y" "Y= " (Utilities|String|ToString(Float) (.y _output_get)) "" 2.0 "(R=0.000000,G=1.000000,B=1.000000,A=1.000000)")
  (Pawn|Input|AddMovementInput (Math|Vector|MakeVector 0.0 (.y _output_get) 0.0) 1.0 false)
  (if (not (Animation|Montage|MontageIsPlaying (Components|SkeletalMesh|GetAnimInstance (Variables|Character|GetMesh)) 0))
    (if (< (Math|Float|Sign(Float) (.y _output_get)) 0.0)
      (Utilities|FlowControl|DoOnce false :!label _label
        (:Completed
          (Transformation|AddRelativeRotation (Variables|Character|GetMesh) "0.000000,180.000000,0.000000" false false)
          (goto _label_2 Reset)))
      (else
        (Utilities|FlowControl|DoOnce true :!label _label_2
          (:Completed
            (Transformation|AddRelativeRotation (Variables|Character|GetMesh) "0.000000,-180.000000,0.000000" false false)
            (goto _label Reset)))))))

(event Custom|Stop%20Wall%20Run
  ;[1 1 1] WallRun
  (Timeline|Wall%20Run%20Duration Stop
    (:Update
      (Variables|/Script/Engine.MovementComponent|SetVelocity (Variables|Character|GetCharacterMovement) (Math|Vector|MakeVector (.x (Variables|/Script/Engine.MovementComponent|GetVelocity (Variables|Character|GetCharacterMovement))) (.y (Variables|/Script/Engine.MovementComponent|GetVelocity (Variables|Character|GetCharacterMovement))) (Variables|Movement|GetWallRunSpeed))))
    (:Finished
      (CallFunction|WallRunCancel))))

(event Custom|Parry
  (bind _desired_location (Variables|Default|GetDesired%20Location))
  ;[1 1 1] Parry Event
  (if (not (Animation|Montage|MontageIsPlaying (Components|SkeletalMesh|GetAnimInstance (Variables|Character|GetMesh)) 0))
    (Variables|Default|SetStateMachine "NewEnumerator4")
    (if (> (Math|Float|Absolute(Float) (.x _desired_location)) (Math|Float|Absolute(Float) (.y _desired_location)))
      ;[0 1 0] TODO: make sphere channel on anim notifier (Change Queue)
      (if (> (.x (Variables|Default|GetDesired%20Location)) 0.0)
        (CallFunction|PrintDebugMessage "Parry" "" "Parry: " "Up" 1.0 "(R=0.000000,G=1.000000,B=1.000000,A=1.000000)")
        (CallFunction|HitscanParry "0.000000,0.000000,1.000000")
        (Animation|Montage|PlayMontage (Variables|Character|GetMesh) "/Game/Assets/Actors/CyberBean/Animation/Montages/ParryUp.ParryUp"
          (:OnCompleted
            _)
          (:OnInterrupted
            _))
        (else
          (CallFunction|PrintDebugMessage "Parry" "" "Parry: " "Down" 1.0 "(R=0.000000,G=1.000000,B=1.000000,A=1.000000)")
          (CallFunction|HitscanParry "0.000000,0.000000,-1.000000")
          (Animation|Montage|PlayMontage (Variables|Character|GetMesh) "/Game/Assets/Actors/CyberBean/Animation/Montages/ParryDown.ParryDown"
            (:OnCompleted
              _)
            (:OnInterrupted
              _))))
      (else
        (if (> (.y (Variables|Default|GetDesired%20Location)) 0.0)
          (CallFunction|PrintDebugMessage "Parry" "" "Parry: " "Right" 1.0 "(R=0.000000,G=1.000000,B=1.000000,A=1.000000)")
          (CallFunction|HitscanParry "0.000000,1.000000,0.000000")
          (else
            (CallFunction|PrintDebugMessage "Parry" "" "Parry: " "Left" 1.0 "(R=0.000000,G=1.000000,B=1.000000,A=1.000000)")
            (CallFunction|HitscanParry "0.000000,-1.000000,0.000000")))
        (Animation|Montage|PlayMontage (Variables|Character|GetMesh) "/Game/Assets/Actors/CyberBean/Animation/Montages/ParrySide.ParrySide"
          (:OnCompleted
            _)
          (:OnInterrupted
            _))))
    (CallFunction|FinishState)))

(event Custom|Wall%20Run%20Cancel
  ;[1 1 1] WallRun
  (CallFunction|StopWallRun)
  (CallFunction|FinishState)
  (Utilities|FlowControl|DoOnce false) ; enters at Reset
)

(event Custom|StartStanceRegenerationLoop
  ;[1 1 1] regeneration Loop
  (Utilities|Time|SetTimerbyEvent (delegate Custom|StanceRegeneration) 0.01 true))

(event Custom|StanceRegeneration
  ;[1 1 1] regeneration Loop
  ;;[1 1 1] only do loop if current stance is not 0
  (if (not (== (Variables|Stats|GetCurrentStance) 0.0))
    ;;[1 1 1] only start if damage delay is gone through
    (if (== (Variables|Stats|GetDamageBreakTimer) (Variables|Default|GetDamageBreakCounter))
      ;;[1 1 1] count if it should be regenerating again
      (bind _output_get (Variables|Default|SetRegCounter (+ (Variables|Default|GetRegCounter) 1)))
      (if (>= _output_get (Variables|Stats|GetRegTimer))
        ;;[1 1 1] add regeneration
        (Variables|Stats|SetCurrentStance (- (Variables|Stats|GetCurrentStance) (Variables|Stats|GetRegStanceAmount)))
        (Variables|Default|SetRegCounter 0))
      (else
        ;;[1 1 1] if not increase damage delay counter
        (Variables|Default|SetDamageBreakCounter (+ (Variables|Default|GetDamageBreakCounter) 1))))))

(event Custom|Dash
  (bind _returnvalue (Transformation|GetActorLocation))
  (bind _desired_location (Variables|Default|GetDesired%20Location))
  ;[1 1 1] Dash, Gate and Setting up Variables
  (Variables|Default|SetStateMachine "NewEnumerator1")
  (Utilities|FlowControl|DoOnce false :!label _label
    (:Completed
      (Variables|Movement|SetDashStartVector (Transformation|GetActorLocation))
      (if (!= (.y _desired_location) 0.0)
        ;;[1 1 1] LineTrace
        (Variables|Movement|SetDash%20Direction%20Vector (Math|Vector|Normalize (Math|Vector|MakeVector 0.0 (.y _desired_location) 0.0)))
        (else
          (Variables|Movement|SetDash%20Direction%20Vector (Math|Vector|Normalize (Math|Vector|MakeVector 0.0 (.y (Variables|/Script/Engine.MovementComponent|GetVelocity (Variables|Character|GetCharacterMovement))) 0.0)))))
      (bind _outhit (Collision|LineTraceByChannel (Variables|Movement|GetDashStartVector) (+ (* (Variables|Movement|GetDash%20Direction%20Vector) (Variables|Movement|GetDash%20Distance)) (Variables|Movement|GetDashStartVector)) "TraceTypeQuery1" false 0 "None"))
      (Variables|Movement|SetDashTraceHitResult _outhit)
      (Animation|Montage|PlayMontage (Variables|Character|GetMesh) "/Game/Assets/Actors/CyberBean/Animation/Montages/Dash.Dash" 0.862069
        (:then
          ;[1 1 1] Vector Logic
          (bind _distancepercantage (Timeline|Timeline PlayFromStart)
            (:Update
              (Utilities|FlowControl|Sequence
                (:then_0
                  (if (not (.bBlockingHit (Collision|BreakHitResult (Variables|Movement|GetDashTraceHitResult))))
                    (Transformation|SetActorLocation (Math|Vector|MakeVector (.x (+ (* (* (Variables|Movement|GetDash%20Direction%20Vector) (Variables|Movement|GetDash%20Distance)) _distancepercantage) (Variables|Movement|GetDashStartVector))) (.y (+ (* (* (Variables|Movement|GetDash%20Direction%20Vector) (Variables|Movement|GetDash%20Distance)) _distancepercantage) (Variables|Movement|GetDashStartVector))) (.z (+ (* (* (Variables|Movement|GetDash%20Direction%20Vector) (Variables|Movement|GetDash%20Distance)) _distancepercantage) (Variables|Movement|GetDashStartVector)))) false false)
                    (else
                      ;[1 1 1] Clamp maximum distance based on hit result of line trace
                      (if (< (.y (.ImpactPoint (Collision|BreakHitResult (Variables|Movement|GetDashTraceHitResult)))) (.y (Variables|Movement|GetDashStartVector)))
                        (Transformation|SetActorLocation (Math|Vector|MakeVector (.x (+ (* (* (Variables|Movement|GetDash%20Direction%20Vector) (Variables|Movement|GetDash%20Distance)) _distancepercantage) (Variables|Movement|GetDashStartVector))) (+ (Math|Float|Clamp(Float) (.y (+ (* (* (Variables|Movement|GetDash%20Direction%20Vector) (Variables|Movement|GetDash%20Distance)) _distancepercantage) (Variables|Movement|GetDashStartVector))) (.y (.ImpactPoint (Collision|BreakHitResult (Variables|Movement|GetDashTraceHitResult)))) (.y _returnvalue)) (Variables|/Script/Engine.CapsuleComponent|GetCapsuleRadius (Variables|Collision|GetCapsuleComponent))) (.z (+ (* (* (Variables|Movement|GetDash%20Direction%20Vector) (Variables|Movement|GetDash%20Distance)) _distancepercantage) (Variables|Movement|GetDashStartVector)))) false false)
                        (else
                          (Transformation|SetActorLocation (Math|Vector|MakeVector (.x (+ (* (* (Variables|Movement|GetDash%20Direction%20Vector) (Variables|Movement|GetDash%20Distance)) _distancepercantage) (Variables|Movement|GetDashStartVector))) (- (Math|Float|Clamp(Float) (.y (+ (* (* (Variables|Movement|GetDash%20Direction%20Vector) (Variables|Movement|GetDash%20Distance)) _distancepercantage) (Variables|Movement|GetDashStartVector))) (.y _returnvalue) (.y (.ImpactPoint (Collision|BreakHitResult (Variables|Movement|GetDashTraceHitResult))))) (Variables|/Script/Engine.CapsuleComponent|GetCapsuleRadius (Variables|Collision|GetCapsuleComponent))) (.z (+ (* (* (Variables|Movement|GetDash%20Direction%20Vector) (Variables|Movement|GetDash%20Distance)) _distancepercantage) (Variables|Movement|GetDashStartVector)))) false false))))))
                (:then_1
                  ;[0 1 0] TODO IFrames
                  (if true
                    _))))
            (:Finished
              (Utilities|FlowControl|Delay (Variables|Movement|GetDashCooldown))
              (CallFunction|PrintDebugMessage "Dash" "" "Dash Resetted" "" 1.0 "(R=0.000000,G=1.000000,B=1.000000,A=1.000000)")
              (CallFunction|FinishState)
              (goto _label Reset))))))))

(event Custom|Attack
  (bind _desired_location (Variables|Default|GetDesired%20Location))
  ;[1 1 1] Attack Event
  (if (not (Animation|Montage|MontageIsPlaying (Components|SkeletalMesh|GetAnimInstance (Variables|Character|GetMesh)) 0))
    (Variables|Default|SetStateMachine "NewEnumerator3")
    (if (> (Math|Float|Absolute(Float) (.x _desired_location)) (Math|Float|Absolute(Float) (.y _desired_location)))
      (if (> (.x (Variables|Default|GetDesired%20Location)) 0.0)
        ;[0 1 0] TODO: make sphere channel on anim notifier (Change Queue)
        (CallFunction|PrintDebugMessage "Attack" "" "Attack: " "Up" 1.0 "(R=0.000000,G=1.000000,B=1.000000,A=1.000000)")
        (CallFunction|HitscanAttack "0.000000,0.000000,1.000000")
        (Animation|Montage|PlayMontage (Variables|Character|GetMesh) "/Game/Assets/Actors/CyberBean/Animation/Montages/UpAttack.UpAttack"
          (:OnCompleted
            _)
          (:OnInterrupted
            _))
        (CallFunction|FinishState :!label _label)
        (elif (not (AI|Components|NavMovement|IsMovingonGround (Variables|Character|GetCharacterMovement)))
          (CallFunction|PrintDebugMessage "Attack" "" " Attack: " "Down" 1.0 "(R=0.000000,G=1.000000,B=1.000000,A=1.000000)")
          (CallFunction|HitscanAttack "0.000000,0.000000,-1.000000")
          (Animation|Montage|PlayMontage (Variables|Character|GetMesh) "/Game/Assets/Actors/CyberBean/Animation/Montages/DownAttack.DownAttack"
            (:OnCompleted
              (goto _label))
            (:OnInterrupted
              (goto _label)))))
      (else
        (if (> (.y (Variables|Default|GetDesired%20Location)) 0.0)
          (CallFunction|PrintDebugMessage "Attack" "" "Attack: " "Right" 1.0 "(R=0.000000,G=1.000000,B=1.000000,A=1.000000)")
          (CallFunction|HitscanAttack "0.000000,1.000000,0.000000")
          (else
            (CallFunction|PrintDebugMessage "Attack" "" "Attack: " "Left" 1.0 "(R=0.000000,G=1.000000,B=1.000000,A=1.000000)")
            (CallFunction|HitscanAttack "0.000000,-1.000000,0.000000")))
        (Animation|Montage|PlayMontage (Variables|Character|GetMesh) "/Game/Assets/Actors/CyberBean/Animation/Montages/SideAttack.SideAttack"
          (:OnCompleted
            (goto _label))
          (:OnInterrupted
            (goto _label)))))))

(event EventTick
  (params (DeltaSeconds :type Float%20%28single-precision%29))
  (CallFunction|PrintDebugMessage "State" "" (Utilities|String|EnumtoString (Variables|Default|GetStateMachine)) "" 1.0 "(R=0.000000,G=1.000000,B=1.000000,A=1.000000)"))

(event EventOnMovementModeChanged
  (params (PrevMovementMode :type EMovementMode%20Enum :default "MOVE_None") (NewMovementMode :type EMovementMode%20Enum :default "MOVE_None") (PrevCustomMode :type Byte :default 0) (NewCustomMode :type Byte :default 0))
  ;[1 1 1] State Machine Jumping to Normal transition
  (if (and (Utilities|Enum|Equal(Enum) PrevMovementMode "MOVE_Falling") (Utilities|Enum|Equal(Enum) NewMovementMode "MOVE_Walking"))
    (Variables|Movement|SetCanRunOnWalls? true)
    (Variables|Default|SetStateMachine "NewEnumerator0")))

(event EventBeginPlay
  (Variables|Stats|SetCurrentHealth (Variables|Stats|GetMaxHealth))
  (CallFunction|StartStanceRegenerationLoop))

(event Input|KeyboardEvents|B
  (params (Key :type Key%20Structure :default "None"))
  ;[1 1 1] damage debug
  (:Pressed
    (bind (_is_dead _isstance _new_health _new_stance) (CallFunction|TakeDamage (Variables|Stats|GetCurrentHealth) 1e+01 (Variables|Stats|GetCurrentStance) 2e+01 (Variables|Stats|GetMaxStance)))
    (Variables|Stats|SetCurrentHealth _new_health)
    (Variables|Stats|SetCurrentStance _new_stance)
    (Variables|Default|SetDamageBreakCounter 0)
    (if _is_dead
      (Development|PrintString "You Dead Bro")
      (elif _isstance
        (Development|PrintString "You CCt")))))

(fn ConstructionScript)

(fn HitscanAttack
  (params (Sphere%20Direction :type Vector))
  (bind _returnvalue (Transformation|GetActorLocation))
  (bind (_outhit _returnvalue_2) (Collision|SphereTraceByChannel _returnvalue (+ _returnvalue (* Sphere%20Direction (Variables|Attack|GetAttackRange))) (Variables|Attack|GetAttack%20Width) "TraceTypeQuery1" false 0 "Persistent"))
  (return _outhit _returnvalue_2 Sphere%20Direction))

(fn HitscanParry
  (params (A :type Vector))
  (bind _returnvalue (Transformation|GetActorLocation))
  (bind (_outhit _returnvalue_2) (Collision|SphereTraceByChannel _returnvalue (+ _returnvalue (* A (Variables|Parry|GetParry%20Range))) (Variables|Parry|GetParry%20Width) "TraceTypeQuery1" false 0 "Persistent"))
  (return _outhit _returnvalue_2))

(fn CustomJump
  (if (Utilities|Enum|Equal(Enum) (Variables|Default|GetStateMachine) "NewEnumerator5")
    (Variables|Default|SetStateMachine "NewEnumerator2")
    (CallFunction|WallJump)
    (else
      (Variables|Default|SetStateMachine "NewEnumerator2")
      (Character|Jump))))

(fn CustomStopJumping
  (CallFunction|PrintDebugMessage "Jump" "Jump: " "Falling" "" 1.0 "(R=0.000000,G=1.000000,B=1.000000,A=1.000000)")
  (if (> (.z (Variables|/Script/Engine.MovementComponent|GetVelocity (Variables|Character|GetCharacterMovement))) (Variables|Movement|GetStopJumpDownwardForce))
    (Variables|/Script/Engine.MovementComponent|SetVelocity (Variables|Character|GetCharacterMovement) (Math|Vector|MakeVector (.x (Variables|/Script/Engine.MovementComponent|GetVelocity (Variables|Character|GetCharacterMovement))) (.y (Variables|/Script/Engine.MovementComponent|GetVelocity (Variables|Character|GetCharacterMovement))) (Variables|Movement|GetStopJumpDownwardForce)))
    (Character|StopJumping)))

(fn FinishState
  (if (AI|Components|NavMovement|IsMovingonGround (Variables|Character|GetCharacterMovement))
    (Variables|Default|SetStateMachine "NewEnumerator0")
    (else
      (Variables|Default|SetStateMachine "NewEnumerator2"))))

(fn WallJump
  (bind _walljumplaunchvector (Variables|Default|GetWallJumpLaunchVector))
  (CallFunction|WallRunCancel)
  (if (< (.y (Transformation|GetWorldLocation (Variables|Movement|GetClimbed%20Object))) (.y (Transformation|GetActorLocation)))
    (Variables|Default|SetDesired%20Location "(X=0.000000,Y=1.000000)")
    (Character|LaunchCharacter (Math|Vector|MakeVector (.x _walljumplaunchvector) (.y _walljumplaunchvector) (.z _walljumplaunchvector)) true true)
    (else
      (Variables|Default|SetDesired%20Location "(X=0.000000,Y=-1.000000)")
      (Character|LaunchCharacter (Math|Vector|MakeVector (.x _walljumplaunchvector) (* (.y _walljumplaunchvector) -1.0) (.z _walljumplaunchvector)) true true))))