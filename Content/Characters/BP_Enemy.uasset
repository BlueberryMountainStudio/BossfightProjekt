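; Enemy character with health and a stance meter that fills by a fixed amount per hit; a hit taken at full stance deals max-health damage.
; A looping timer drains stance after a post-hit delay, which each normal hit rescales by missing health up to a cap.
; Health and stance percentages and death are written to BP_MCPC, the player controller, and the actor destroys itself on death.
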(event Custom|StartStanceRegenerationLoop
  ;[1 1 1] regeneration Loop
  (Utilities|Time|SetTimerbyEvent (delegate Custom|StanceRegeneration) 0.01 true))

(event Custom|StanceRegeneration
  ;[1 1 1] regeneration Loop
  ;;[0.9569 1 0.09804] only do loop if current stance is not 0
  (if (not (== (Variables|Stats|GetCurrentStance) 0.0))
    ;;[0.9569 1 0.09804] only start if damage delay is gone through
    (if (== (Variables|Stats|GetDamage%20Break%20Timer) (Variables|Default|GetDamage%20Break%20Counter))
      ;;[0.9569 1 0.09804] count if it should be regenerating again
      (bind _output_get (Variables|Default|SetRegCounter (+ (Variables|Default|GetRegCounter) 1)))
      (if (>= _output_get (Variables|Stats|GetRegTimer))
        ;;[0.9569 1 0.09804] add regeneration
        (Variables|Stats|SetCurrentStance (- (Variables|Stats|GetCurrentStance) (Variables|Stats|GetRegStanceAmount)))
        (Variables|Default|SetRegCounter 0)
        (CallFunction|UpdateStancePercent))
      (else
        ;;[0.9569 1 0.09804] if not increase damage delay counter
        (Variables|Default|SetDamage%20Break%20Counter (+ (Variables|Default|GetDamage%20Break%20Counter) 1))))))

(event EventBeginPlay
  (bind _asbp_mcpc (Utilities|Casting|CastToBP_MCPC (Game|GetPlayerController 0)))
  (Variables|References|SetController_Ref _asbp_mcpc)
  (Variables|Stats|SetCurrentHealth (Variables|Stats|GetMaxHealth))
  (CallFunction|StartStanceRegenerationLoop)
  (CallFunction|UpdateHealthPercent)
  (CallFunction|UpdateStancePercent))

(event Game|Damage|EventAnyDamage
  (params (Damage :type Float%20%28single-precision%29) (DamageType :type Damage%20Type%20Object%20Reference) (InstigatedBy :type Controller%20Object%20Reference) (DamageCauser :type Actor%20Object%20Reference))
  (bind _maxhealth (Variables|Stats|GetMaxHealth))
  ;[1 1 1] event take damage
  (if (>= (Variables|Stats|GetCurrentStance) (Variables|Stats|GetMaxStance))
    (Development|PrintString "Stance Kill" true true "(R=1.000000,G=0.538961,B=0.000000,A=1.000000)")
    (bind (_is_dead _isstance _new_health _new_stance) (CallFunction|TakeDamage (Variables|Stats|GetCurrentHealth) (Variables|Stats|GetMaxHealth) (Variables|Stats|GetCurrentStance) 0.0 (Variables|Stats|GetMaxStance)))
    (Variables|Stats|SetCurrentHealth _new_health)
    (Variables|Stats|SetCurrentStance _new_stance)
    (Variables|Default|SetIsDead _is_dead)
    (else
      (bind (_is_dead_2 _isstance_2 _new_health_2 _new_stance_2) (CallFunction|TakeDamage (Variables|Stats|GetCurrentHealth) Damage (Variables|Stats|GetCurrentStance) 4e+01 (Variables|Stats|GetMaxStance)))
      (bind _output_get (Variables|Stats|SetCurrentHealth _new_health_2))
      (Variables|Stats|SetCurrentStance _new_stance_2)
      (Variables|Default|SetIsDead _is_dead_2)
      ;;[0.1333 0.9255 1] check if damage break timer has reached maximum
      (if (< (Variables|Stats|GetDamage%20Break%20Timer) (Variables|Stats|GetMaxDamageBreak))
        ;;[0.1333 0.9255 1] multiply with damage break timer to increase it
        (Variables|Stats|SetDamage%20Break%20Timer (Math|Float|Truncate (* (* (/ (- _maxhealth _output_get) _maxhealth) (Variables|Stats|GetMultiplyMissingPercent)) (Variables|Stats|GetDamage%20Break%20Timer))))
        ;;[0.1333 0.9255 1] if damage break timer went over max value set it back to max value
        (if (< (Variables|Stats|GetDamage%20Break%20Timer) (Variables|Stats|GetMaxDamageBreak))
          _
          (else
            (bind _output_get_2 (Variables|Stats|SetDamage%20Break%20Timer (Variables|Stats|GetMaxDamageBreak))))))
      (CallFunction|PrintDebugMessage "None" "Damage Break Timer: " (Utilities|String|ToString(Integer) _output_get_2) "ms" 2.0 "(R=0.751597,G=0.169159,B=1.000000,A=1.000000)")))
  (Variables|Default|SetDamage%20Break%20Counter 0)
  (CallFunction|UpdateHealthPercent)
  (CallFunction|UpdateStancePercent)
  (if (Variables|Default|GetIsDead)
    (Variables|/Game/Game/BP_MCPC.BP_MCPC_C|SetEnemyDead (Variables|References|GetController_Ref) (Variables|Default|GetIsDead))
    (Actor|DestroyActor)))

(fn ConstructionScript)

(fn UpdateHealthPercent
  (Variables|/Game/Game/BP_MCPC.BP_MCPC_C|SetEnemyHealthPercent (Variables|References|GetController_Ref) (/ (Variables|Stats|GetCurrentHealth) (Variables|Stats|GetMaxHealth)))
  (return))

(fn UpdateStancePercent
  (Variables|/Game/Game/BP_MCPC.BP_MCPC_C|SetEnemyStancePercent (Variables|References|GetController_Ref) (/ (Variables|Stats|GetCurrentStance) (Variables|Stats|GetMaxStance)))
  (return))