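; BP_Theme is an actor that plays a theme audio track for the map through its Audio component.
; On BeginPlay it sets starting Volume and Fade Time float parameters on the sound, then plays it.
; SetVolume and SetFadeTime events update those parameters at runtime, with comments indicating box collision as the intended caller.
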(event EventBeginPlay
  (bind _audio (Variables|Default|GetAudio))
  ;[1 1 1] Set Start Audio-Values
  (Components|Activation|Activate _audio false)
  (Audio|Parameter|SetFloatParameter _audio "Volume" 0.2 :!class /Script/Engine.AudioComponent)
  (Audio|Parameter|SetFloatParameter _audio "Fade Time" 3.0 :!class /Script/Engine.AudioComponent)
  (Audio|Components|Audio|Play _audio 0.0))

(event EventSetVolume
  (params (Volume :type Float%20%28double-precision%29))
  ;[1 1 1] Set Volume (BoxCollision)
  (Audio|Parameter|SetFloatParameter (Variables|Default|GetAudio) "Volume" Volume :!class /Script/Engine.AudioComponent))

(event EventSetFadeTime
  (params (FadeTime :type Float%20%28double-precision%29))
  ;[1 1 1] Set Volume Fade Time (BoxCollision)
  (Audio|Parameter|SetFloatParameter (Variables|Default|GetAudio) "Fade Time" FadeTime :!class /Script/Engine.AudioComponent))

(fn ConstructionScript)